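; GodMode is a debug cheat component whose GodMode flag gates helpers to spawn actors, destroy all actors of a class, and open AssetLevel on the tenth A press.
; Key input builds a string and collects cheats containing it into PossibleCheats, without triggering them.
; An older letter-by-letter matcher that toggled the flag is left unconnected.
; BeginPlay concatenates configured strings into MyBonuses.
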(event `self.ReceiveBeginPlay`
  (for _index (range (+ (* (`self.String Number`) 2) 1))
    (set `self.MyBonuses` (`KismetStringLibrary.Concat_StrStr` (`self.MyBonuses`) (select `int` _index :`0` "" :`1` (`self.First String`) :`2` "" :`3` (`self.Second String`) :`4` "" :`5` (`self.Third String`) :`6` "" :`7` (`self.Fourth String`) :`8` "" :`9` (`self.Fifth String`) :`10` "" :`11` (`self.Sixth String`) :`12` "" :`13` (`self.Seventh String`) :`14` "" :`15` (`self.Eight String`) :`16` "" :`17` (`self.Ninth String`) :`18` "" :`19` (`self.Tenth String`) :`20` "" :`21` (`self.Eleven String`) :`22` "" :`23` (`self.Twelve String`))))))

(fn `Activate/Deactivate God Mode`
  (params (Key :type "Key Structure" :default "None"))
  (`self.Verify String Wrote` Key (`self.Cheats`)))

(fn `B`
  (params (Key :type "Key Structure" :default "None"))
  (returns (`Correct Key` :type Boolean))
  (if (== Key "B")
    (set `self.B_` true)
    (return true)
    (else
      (`self.Reset all Letter`)
      (return false))))

(fn `Change God Mode`
  (set `self.God Mode` (not (`self.God Mode`))))

(fn `D`
  (params (Key :type "Key Structure" :default "None"))
  (returns (`Correct Key` :type Boolean))
  (if (== Key "D")
    (set `self.D_` true)
    (return true)
    (else
      (`self.Reset all Letter`)
      (return false))))

(fn `Destroy all Object Reference`
  (params (ActorClass :type "Actor Class Reference"))
  (if (`self.God Mode`)
    (bind _outactors (`GameplayStatics.GetAllActorsOfClass` ActorClass))
    (for _array_element _outactors
      (`Actor.K2_DestroyActor` _array_element))))

(fn `G`
  (params (Key :type "Key Structure" :default "None"))
  (returns (`Correct Key` :type Boolean))
  (if (== Key "G")
    (set `self.G_` true)
    (return true)
    (else
      (`self.Reset all Letter`)
      (return false))))

(fn `M`
  (params (Key :type "Key Structure" :default "None"))
  (returns (`Correct Key` :type Boolean))
  (if (== Key "M")
    (set `self.M_` true)
    (return true)
    (else
      (`self.Reset all Letter`)
      (return false))))

(fn `O`
  (params (Key :type "Key Structure" :default "None"))
  (returns (`Correct Key` :type Boolean))
  (if (== Key "O")
    (set `self.O_` true)
    (return true)
    (else
      (`self.Reset all Letter`)
      (return false))))

(fn `Reset all Letter`
  (set `self.G_` false)
  (set `self.O_` false)
  (set `self.D_` false)
  (set `self.Space_` false)
  (set `self.M_` false)
  (set `self.B_` false))

(fn `Set Letter Number 0 `
  (set `self.Letter number` 0))

(fn `Space`
  (params (Key :type "Key Structure" :default "None"))
  (returns (`Correct Key` :type Boolean))
  (if (== Key "SpaceBar")
    (set `self.Space_` true)
    (return true)
    (else
      (`self.Reset all Letter`)
      (return false))))

(fn `Spawn Object`
  (params (Class :type "Actor Class Reference") (`Spawn Transform Location` :type "Vector Structure"))
  (if (`self.God Mode`)
    (`|SpawnActorFromClass` Class (`KismetMathLibrary.MakeTransform` `Spawn Transform Location`) "Undefined" "OverrideRootScale" null null)))

(fn `Teleport To Asset Level`
  (params (Key :type "Key Structure" :default "None"))
  (bind _counter_letter (`self.Counter Letter`))
  (if (`self.God Mode`)
    (if (== Key "A")
      (`/Engine/EditorBlueprintResources/StandardMacros.IncrementInt` _counter_letter
        (:`  `
          (if (== _counter_letter 10)
            (set `self.Counter Letter` 0)
            (`GameplayStatics.OpenLevel` "AssetLevel")
            (else
              (`KismetSystemLibrary.PrintString` (`KismetStringLibrary.Conv_IntToString` _counter_letter) true true (struct :`G` 0.66 :`B` 1.0 :`A` 1.0) 0.0))))))))

(fn `Verify String Wrote`
  (params (Key :type "Key Structure" :default "None") (Cheats :type "Array of String"))
  (set `self.MyCheat` (`KismetStringLibrary.Concat_StrStr` (`KismetTextLibrary.Conv_TextToString` (`KismetInputLibrary.Key_GetDisplayName` Key)) (`self.MyCheat`)))
  (for _array_element Cheats
    (if (`KismetStringLibrary.Contains` _array_element (`self.MyCheat`))
      (if (not (`KismetArrayLibrary.Array_Contains` (`self.Possible Cheats`) _array_element))
        (`KismetArrayLibrary.Array_Add` (`self.Possible Cheats`) _array_element)))))