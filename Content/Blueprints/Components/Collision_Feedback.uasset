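; Collision feedback component that tracks whether it is touching a player, a human or an interactible object.
; StartTouching overwrites all three flags with type checks on the incoming entity, so only the latest contact counts.
; EndTouching clears flags matching the departing entity's type and returns them with that entity as an interactible object.
; GetObject is an empty stub, and the event graph is unused.
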(fn `EndTouching`
  (params (Entity :type "Object Object Reference"))
  (returns (`Is Touching Player` :type Boolean) (`Is Touching Human` :type Boolean) (`Is Touching Interactible Object` :type Boolean) (`As Interactible Object` :type "/Game/Blueprints/Entities/InteractibleObjects/InteractibleObject Object Reference"))
  (bind (_as_interactible_object _success) (`/Game/Blueprints/Managers/Library.Is Interactible Object` Entity))
  (if (and (`self.Is Touching Player`) (`.Success` (`/Game/Blueprints/Managers/Library.Is Player` Entity)))
    (set `self.Is Touching Player` false))
  (if (and (`self.Is Touching Human`) (`.Success` (`/Game/Blueprints/Managers/Library.Is Human` Entity)))
    (set `self.Is Touching Human` false))
  (if (and _success (`self.Is Touching Interactible Object`))
    (set `self.Is Touching Interactible Object` false))
  (return (`self.Is Touching Player`) (`self.Is Touching Human`) (`self.Is Touching Interactible Object`) _as_interactible_object))

(fn `Get Object`)

(fn `StartTouching`
  (params (Entity :type "Object Object Reference"))
  (returns (`Is Touching Player` :type Boolean) (`Is Touching Human` :type Boolean) (`Is Touching Interactible Object` :type Boolean))
  (set `self.Is Touching Player` (`.Success` (`/Game/Blueprints/Managers/Library.Is Player` Entity)))
  (set `self.Is Touching Human` (`.Success` (`/Game/Blueprints/Managers/Library.Is Human` Entity)))
  (set `self.Is Touching Interactible Object` (`.Success` (`/Game/Blueprints/Managers/Library.Is Interactible Object` Entity)))
  (return (`self.Is Touching Player`) (`self.Is Touching Human`) (`self.Is Touching Interactible Object`)))