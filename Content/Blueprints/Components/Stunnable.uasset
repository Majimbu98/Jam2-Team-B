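; Stunnable component that handles a player being stunned by a human and the player's invincibility.
; StunnedByHuman acts only when the player is idle or transforming an object, resetting that object to its starting state in the latter case before applying the stun.
; BecomeInvincible, which requests a delay reset, and FinishImmunity pass straight through to the state processor, which handles all state changes.
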(fn `Become Invincible`
  (params (Player :type "/Game/Blueprints/Entities/Player/Player Object Reference"))
  (`/Game/Blueprints/Managers/StateProcessor.(Player)Become Invincible` (`/Game/Blueprints/Managers/Library.Get State Processor`) Player true))

(fn `FinishImmunity`
  (params (Player :type "/Game/Blueprints/Entities/Player/Player Object Reference"))
  (`/Game/Blueprints/Managers/StateProcessor.(Player)Finish Immunity` (`/Game/Blueprints/Managers/Library.Get State Processor`) Player))

(fn `Stunned by Human`
  (params (Player :type "/Game/Blueprints/Entities/Player/Player Object Reference") (Object :type "/Game/Blueprints/Entities/InteractibleObjects/InteractibleObject Object Reference"))
  (switch `/Game/Blueprints/Entities/Player/PlayerStates/PlayerStates` (`/Game/Blueprints/Entities/Player/Player.State` Player)
    (:`NewEnumerator0`
      _)
    (:`NewEnumerator1`
      (`/Game/Blueprints/Managers/StateProcessor.(Interactible Object)Set Interactible Object Starting State` (`/Game/Blueprints/Managers/Library.Get State Processor`) Object)))
  (`/Game/Blueprints/Managers/StateProcessor.(Player)Stunned By Human` (`/Game/Blueprints/Managers/Library.Get State Processor`) Player))