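; WavesManager is a wave manager that spawns Human actors according to the current MainWave index.
; Activate and NextWave, which increments the index, share one switch: wave 0 spawns humans in a WavesSize loop at the origin, wave 1 zeroes WavesSize.
; SpawnHuman assigns a random skeletal mesh from MeshList and has the state processor set the starting state.
; Tick and the overlap event's SpawnPointHuman lookup have no effect.
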(event `self.ReceiveTick`
  (params (DeltaSeconds :type "Float (single-precision)"))
  (`|ExecutionSequence`))

(event `self.ReceiveActorBeginOverlap`
  (params (OtherActor :type "Actor Object Reference"))
  (`GameplayStatics.GetAllActorsOfClass` "/Game/Blueprints/Entities/IA/SpawnPointHuman.SpawnPointHuman_C"))

(event `Activate`
  ;[1 1 1] Cose
  (switch `int` (`self.Main Wave`) :!label _label
    (:`0`
      (for _ (range (+ (stale _output_get) 1))
        (`self.Spawn Human` (0.0 0.0 0.0))))
    (:`1`
      (bind _output_get (set `self.WavesSize` 0)))))

(event `Next Wave`
  (`/Engine/EditorBlueprintResources/StandardMacros.IncrementInt` (`self.Main Wave`)
    (:`  `
      (goto _label))))

(fn `Spawn Human`
  (params (`Human Position` :type "Vector Structure"))
  (bind _returnvalue (`|SpawnActorFromClass` "/Game/Blueprints/Entities/IA/Human.Human_C" (`KismetMathLibrary.Conv_VectorToTransform` `Human Position`) "Undefined" "OverrideRootScale" null null))
  (`SkinnedMeshComponent.SetSkinnedAssetAndUpdate` (`Character.Mesh` _returnvalue) (`KismetArrayLibrary.Array_Random` (`self.Mesh List`)) true)
  (`/Game/Blueprints/Managers/StateProcessor.(Human)Set Starting Human State` (`/Game/Blueprints/Managers/Library.Get State Processor`) _returnvalue))

(fn `UserConstructionScript`)