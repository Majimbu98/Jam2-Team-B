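; StateProcessor is a manager that runs state transitions for the player, interactible objects that can turn scary, and humans.
; It uses an actor-based state pattern: most transitions destroy the attached state actor, set an enum, then spawn, attach and often activate a new one.
; Player transform start and stop also drive object scare states, branching on invincibility, Space release and whether a human is checking, which stuns the player.
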(event `Set Interactible Object`
  (for _array_element (`/Game/Blueprints/Managers/Library.Get InteractibleObjects`)
    (`self.(Interactible Object)Set Interactible Object Starting State` _array_element))
  (`self.(Player)Set Starting Player State` (`/Game/Blueprints/Managers/Library.Get Player`)))

(fn `(Human) Set Starting Human State`
  (params (Human :type "/Game/Blueprints/Entities/IA/Human Object Reference"))
  (`/Engine/EditorBlueprintResources/StandardMacros.IsValid` (`|GetArrayItem` (`self.GetAttachedActors` Human true))
    (:`Is Valid`
      (`/Game/Blueprints/Managers/Library.Destroy Attached actor` Human))
    (:`Is Not Valid`
      _))
  (set `/Game/Blueprints/Entities/IA/Human.State` "NewEnumerator0" Human)
  (bind _returnvalue (`|SpawnActorFromClass` "/Game/Blueprints/Entities/IA/States/Waiting.Waiting_C" (`SceneComponent.K2_GetComponentToWorld` (`Actor.RootComponent` Human)) "Undefined" "OverrideRootScale" null null))
  (`self.K2_AttachToActor` _returnvalue Human "WaitingState" "KeepRelative" "KeepRelative" "KeepRelative" true)
  (`/Game/Blueprints/Entities/IA/States/Waiting.Activate` _returnvalue Human))

(fn `(Interactible Object) Becoming Scary`
  (params (`Interactible Object` :type "/Game/Blueprints/Entities/InteractibleObjects/InteractibleObject Object Reference") (Player :type "/Game/Blueprints/Entities/Player/Player Object Reference"))
  (`/Game/Blueprints/Managers/Library.Destroy Attached actor` `Interactible Object`)
  (set `/Game/Blueprints/Components/Interactible.State` "NewEnumerator1" (`/Game/Blueprints/Entities/InteractibleObjects/InteractibleObject.Interactible` `Interactible Object`))
  (`/Game/Blueprints/Entities/InteractibleObjects/InteractibleObject.Change Mesh` `Interactible Object`)
  (bind _returnvalue (`|SpawnActorFromClass` "/Game/Blueprints/Entities/InteractibleObjects/States/BecomingScary.BecomingScary_C" (`SceneComponent.K2_GetComponentToWorld` (`/Game/Blueprints/Entities/InteractibleObjects/InteractibleObject.DefaultSceneRoot` `Interactible Object`)) "Undefined" "OverrideRootScale" null null))
  (`self.K2_AttachToActor` _returnvalue `Interactible Object` "BecomingScaryState" "KeepRelative" "KeepRelative" "KeepRelative" true)
  (`/Game/Blueprints/Entities/InteractibleObjects/States/BecomingScary.Activate` _returnvalue `Interactible Object` Player))

(fn `(Interactible Object)Coming Back To Scary`
  (params (Player :type "/Game/Blueprints/Entities/Player/Player Object Reference") (`Interactible Object` :type "/Game/Blueprints/Entities/InteractibleObjects/InteractibleObject Object Reference"))
  (locals (`Player Ref` :type "/Game/Blueprints/Entities/Player/Player Object Reference") (`Interactible Object Ref` :type "/Game/Blueprints/Entities/InteractibleObjects/InteractibleObject Object Reference"))
  (bind _interactible_object_ref (`local.Interactible Object Ref`))
  (bind _interactible_object_ref_2 (`local.Interactible Object Ref`))
  (`|VariableSetRef` (`local.Player Ref`) Player)
  (`|VariableSetRef` _interactible_object_ref_2 `Interactible Object`)
  (`/Game/Blueprints/Managers/Library.Destroy Attached actor` _interactible_object_ref_2)
  (set `/Game/Blueprints/Components/Interactible.State` "NewEnumerator3" (`/Game/Blueprints/Entities/InteractibleObjects/InteractibleObject.Interactible` _interactible_object_ref))
  (`/Game/Blueprints/Entities/InteractibleObjects/InteractibleObject.Change Mesh` _interactible_object_ref)
  (bind _returnvalue (`|SpawnActorFromClass` "/Game/Blueprints/Entities/InteractibleObjects/States/ComingBackToScary.ComingBackToScary_C" (`SceneComponent.K2_GetComponentToWorld` (`/Game/Blueprints/Entities/InteractibleObjects/InteractibleObject.DefaultSceneRoot` _interactible_object_ref)) "Undefined" "OverrideRootScale" null null))
  (`self.K2_AttachToActor` _returnvalue _interactible_object_ref "ComingBackToScaryState" "KeepRelative" "KeepRelative" "KeepRelative" true)
  (`/Game/Blueprints/Entities/InteractibleObjects/States/ComingBackToScary.Activate` _returnvalue _interactible_object_ref (`local.Player Ref`)))

(fn `(Interactible Object)Scary CountDown`
  (params (`Interactible Object` :type "/Game/Blueprints/Entities/InteractibleObjects/InteractibleObject Object Reference") (`Was Scary?` :type Boolean) (Player :type "/Game/Blueprints/Entities/Player/Player Object Reference"))
  (`/Game/Blueprints/Managers/Library.Destroy Attached actor` `Interactible Object`)
  (bind _returnvalue (`|SpawnActorFromClass` "/Game/Blueprints/Entities/InteractibleObjects/States/Scary.Scary_C" (`SceneComponent.K2_GetComponentToWorld` (`/Game/Blueprints/Entities/InteractibleObjects/InteractibleObject.DefaultSceneRoot` `Interactible Object`)) "Undefined" "OverrideRootScale" null null))
  (`self.K2_AttachToActor` _returnvalue `Interactible Object` "Scary State" "KeepRelative" "KeepRelative" "KeepRelative" true)
  (`/Game/Blueprints/Entities/InteractibleObjects/States/Scary.Activate` _returnvalue `Interactible Object` `Was Scary?` Player))

(fn `(Interactible Object)Set Interactible Object Starting State`
  (params (Object :type "/Game/Blueprints/Entities/InteractibleObjects/InteractibleObject Object Reference"))
  (`/Engine/EditorBlueprintResources/StandardMacros.IsValid` (`|GetArrayItem` (`self.GetAttachedActors` Object true))
    (:`Is Valid`
      (`/Game/Blueprints/Managers/Library.Destroy Attached actor` Object))
    (:`Is Not Valid`
      _))
  (set `/Game/Blueprints/Components/Interactible.State` "NewEnumerator0" (`/Game/Blueprints/Entities/InteractibleObjects/InteractibleObject.Interactible` Object))
  (set `/Game/Blueprints/Components/Interactible.Time Passed ScaryDuration` 0.0 (`/Game/Blueprints/Entities/InteractibleObjects/InteractibleObject.Interactible` Object))
  (`/Game/Blueprints/Entities/InteractibleObjects/InteractibleObject.Change Mesh` Object)
  (bind _returnvalue (`|SpawnActorFromClass` "/Game/Blueprints/Entities/InteractibleObjects/States/NotScary.NotScary_C" (`SceneComponent.K2_GetComponentToWorld` (`/Game/Blueprints/Entities/InteractibleObjects/InteractibleObject.DefaultSceneRoot` Object)) "Undefined" "OverrideRootScale" null null))
  (`self.K2_AttachToActor` _returnvalue Object "NotScaryState" "KeepRelative" "KeepRelative" "KeepRelative" true))

(fn `(Player)Become Invincible`
  (params (Player :type "/Game/Blueprints/Entities/Player/Player Object Reference") (`Reset Delay?` :type Boolean))
  (locals (`Player Ref` :type "/Game/Blueprints/Entities/Player/Player Object Reference"))
  (bind _player_ref (`local.Player Ref`))
  (`|VariableSetRef` _player_ref Player)
  (`/Game/Blueprints/Managers/Library.Destroy Attached actor` _player_ref)
  (set `/Game/Blueprints/Entities/Player/Player.State` "NewEnumerator3" _player_ref)
  (bind _returnvalue (`|SpawnActorFromClass` "/Game/Blueprints/Entities/Player/PlayerStates/InvincibleState.InvincibleState_C" (`self.GetTransform` _player_ref) "Undefined" "OverrideRootScale" null null))
  (`self.K2_AttachToActor` _returnvalue _player_ref "InvincibleState" "KeepRelative" "KeepRelative" "KeepRelative" true)
  (`/Game/Blueprints/Entities/Player/PlayerStates/InvincibleState.Activate` _returnvalue _player_ref `Reset Delay?`))

(fn `(Player)Finish Immunity`
  (params (Player :type "/Game/Blueprints/Entities/Player/Player Object Reference"))
  (`/Game/Blueprints/Managers/Library.Destroy Attached actor` Player)
  (switch `/Game/Blueprints/Entities/Player/PlayerStates/PlayerStates` (`/Game/Blueprints/Entities/Player/Player.State` Player)
    (:`NewEnumerator4`
      (set `/Game/Blueprints/Entities/Player/Player.State` "NewEnumerator1" Player)
      (bind _returnvalue (`|SpawnActorFromClass` "/Game/Blueprints/Entities/Player/PlayerStates/TrasformingAnObjectState.TrasformingAnObjectState_C" (`SceneComponent.K2_GetComponentToWorld` (`Actor.RootComponent` Player)) "Undefined" "OverrideRootScale" null null))
      (`self.K2_AttachToActor` _returnvalue Player "TrasformingAnObject" "KeepRelative" "KeepRelative" "KeepRelative" true))
    (:`NewEnumerator3`
      (`self.(Player)Set Starting Player State` Player))))

(fn `(Player)Set Starting Player State`
  (params (Player :type "/Game/Blueprints/Entities/Player/Player Object Reference"))
  (`/Engine/EditorBlueprintResources/StandardMacros.IsValid` (`|GetArrayItem` (`self.GetAttachedActors` Player true))
    (:`Is Valid`
      (`/Game/Blueprints/Managers/Library.Destroy Attached actor` Player))
    (:`Is Not Valid`
      _))
  (set `/Game/Blueprints/Entities/Player/Player.State` "NewEnumerator0" Player)
  (bind _returnvalue (`|SpawnActorFromClass` "/Game/Blueprints/Entities/Player/PlayerStates/IdleState.IdleState_C" (`SceneComponent.K2_GetComponentToWorld` (`self.DefaultSceneRoot`)) "Undefined" "OverrideRootScale" null null))
  (`self.K2_AttachToActor` _returnvalue Player "Idle State" "KeepRelative" "KeepRelative" "KeepRelative" true))

(fn `(Player)Start Trasform into Scary Object`
  (params (Object :type "/Game/Blueprints/Entities/InteractibleObjects/InteractibleObject Object Reference") (Player :type "/Game/Blueprints/Entities/Player/Player Object Reference"))
  (bind _interactible (`/Game/Blueprints/Entities/InteractibleObjects/InteractibleObject.Interactible` Object))
  (bind _returnvalue (`SceneComponent.K2_GetComponentToWorld` (`Actor.RootComponent` Player)))
  (if (`/Game/Blueprints/Entities/InteractibleObjects/InteractibleObject.An Human Is Checking` Object)
    (`/Game/Blueprints/Components/Stunnable.Stunned by Human` (`/Game/Blueprints/Entities/Player/Player.Stunnable` Player) Player (`.Interactible Object` (`/Game/Blueprints/Components/Collision_Feedback.Get Interactible Object` (`/Game/Blueprints/Entities/Player/Player.Collision_Feedback` Player))))
    (else
      (`GameplayStatics.PlaySoundAtLocation` "/Game/Audio/SoundEffects/interaction_.interaction_" (`SceneComponent.K2_GetComponentLocation` (`/Game/Blueprints/Entities/Player/Player.Camera` Player)) (struct) 1.0 1.0 0.0 null null null)
      (switch `/Game/Blueprints/Entities/Player/PlayerStates/PlayerStates` (`/Game/Blueprints/Entities/Player/Player.State` Player)
        (:`NewEnumerator0`
          (`/Game/Blueprints/Managers/Library.Destroy Attached actor` Player)
          (set `/Game/Blueprints/Entities/Player/Player.State` "NewEnumerator1" Player)
          (bind _returnvalue_2 (`|SpawnActorFromClass` "/Game/Blueprints/Entities/Player/PlayerStates/TrasformingAnObjectState.TrasformingAnObjectState_C" _returnvalue "Undefined" "OverrideRootScale" null null))
          (`self.K2_AttachToActor` _returnvalue_2 Player "TrasformingAnObjectState" "KeepRelative" "KeepRelative" "KeepRelative" true)
          (switch `/Game/Blueprints/Entities/InteractibleObjects/States/ObjectStates` (`/Game/Blueprints/Components/Interactible.State` (`/Game/Blueprints/Entities/InteractibleObjects/InteractibleObject.Interactible` Object))
            (:`NewEnumerator0`
              (`/Game/Blueprints/Components/Interactible.Becoming Scary` _interactible Object Player :!label _label))
            (:`NewEnumerator2`
              (`/Game/Blueprints/Components/Interactible.Coming Back To Scary` _interactible Player Object :!label _label_2))))
        (:`NewEnumerator3`
          (`/Game/Blueprints/Managers/Library.Destroy Attached actor` Object)
          (set `/Game/Blueprints/Entities/Player/Player.State` "NewEnumerator4" Player)
          (bind _returnvalue_3 (`|SpawnActorFromClass` "/Game/Blueprints/Entities/Player/PlayerStates/TrasformingAnObjectWhileInvincibleState.TrasformingAnObjectWhileInvincibleState_C" _returnvalue "Undefined" "OverrideRootScale" null null))
          (`self.K2_AttachToActor` _returnvalue_3 Player "TrasformingAnObjectWhileInvincibleState" "KeepRelative" "KeepRelative" "KeepRelative" true)
          (switch `/Game/Blueprints/Entities/InteractibleObjects/States/ObjectStates` (`/Game/Blueprints/Components/Interactible.State` (`/Game/Blueprints/Entities/InteractibleObjects/InteractibleObject.Interactible` Object))
            (:`NewEnumerator0`
              (goto _label))
            (:`NewEnumerator2`
              (goto _label_2))))))))

(fn `(Player)StopTransform into ScaryObject`
  (params (object :type "/Game/Blueprints/Entities/InteractibleObjects/InteractibleObject Object Reference") (Player :type "/Game/Blueprints/Entities/Player/Player Object Reference") (`Release "SPACE"` :type Boolean))
  (locals (`Player Ref` :type "/Game/Blueprints/Entities/Player/Player Object Reference") (`Interactible Object Ref` :type "/Game/Blueprints/Entities/InteractibleObjects/InteractibleObject Object Reference"))
  (bind _player_ref (`local.Player Ref`))
  (bind _interactible_object_ref (`local.Interactible Object Ref`))
  (`|VariableSetRef` _player_ref Player)
  (`|VariableSetRef` _interactible_object_ref object)
  (switch `/Game/Blueprints/Entities/InteractibleObjects/States/ObjectStates` (`/Game/Blueprints/Components/Interactible.State` (`/Game/Blueprints/Entities/InteractibleObjects/InteractibleObject.Interactible` _interactible_object_ref))
    (:`NewEnumerator0`
      (switch `/Game/Blueprints/Entities/Player/PlayerStates/PlayerStates` (`/Game/Blueprints/Entities/Player/Player.State` _player_ref) :!label _label
        (:`NewEnumerator1`
          (`self.(Player)Set Starting Player State` _player_ref))
        (:`NewEnumerator4`
          (`self.(Player)Become Invincible` _player_ref))))
    (:`NewEnumerator1`
      (if `Release "SPACE"`
        (`self.(Interactible Object)Set Interactible Object Starting State` _interactible_object_ref)
        (goto _label)
        (else
          (`/Game/Blueprints/Components/Interactible.CountDown Scary Duration` (`/Game/Blueprints/Entities/InteractibleObjects/InteractibleObject.Interactible` _interactible_object_ref) _interactible_object_ref false _player_ref :!label _label_2)
          (goto _label))))
    (:`NewEnumerator2`
      (if `Release "SPACE"`
        (goto _label)
        (else
          (goto _label_2))))
    (:`NewEnumerator3`
      (if `Release "SPACE"`
        (`|ExecutionSequence`
          (:`then_0`
            (`/Game/Blueprints/Components/Interactible.CountDown Scary Duration` (`/Game/Blueprints/Entities/InteractibleObjects/InteractibleObject.Interactible` _interactible_object_ref) _interactible_object_ref true _player_ref))
          (:`then_1`
            (goto _label)))
        (else
          (goto _label))))))

(fn `(Player)Stunned By Human`
  (params (Player :type "/Game/Blueprints/Entities/Player/Player Object Reference"))
  (`/Game/Blueprints/Managers/Library.Destroy Attached actor` Player)
  (set `/Game/Blueprints/Entities/Player/Player.State` "NewEnumerator2" Player)
  (bind _returnvalue (`|SpawnActorFromClass` "/Game/Blueprints/Entities/Player/PlayerStates/StunnedState.StunnedState_C" (`SceneComponent.K2_GetComponentToWorld` (`Actor.RootComponent` Player)) "Undefined" "OverrideRootScale" null null))
  (`self.K2_AttachToActor` _returnvalue Player "Stunned" "KeepRelative" "KeepRelative" "KeepRelative" true)
  (`/Game/Blueprints/Entities/Player/PlayerStates/StunnedState.Activate` _returnvalue Player))

(fn `UserConstructionScript`)