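; Shared helper library that gives gameplay code type checks and lookups for key actors such as the player, GM, managers, state processor and interactible objects.
; Lookups scan the world with GetAllActorsOfClass on each call, most returning the first match.
; It also filters objects that humans can choose, picks a random north or south human spawn point, and destroys an actor's first attached actor.
; The wall check is a stub that always fails.
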(fn `Destroy Attached actor`
  (params (Target :type "Actor Object Reference"))
  (bind _output (`|GetArrayItem` (`Actor.GetAttachedActors` Target true)))
  (`/Engine/EditorBlueprintResources/StandardMacros.IsValid` _output
    (:`Is Valid`
      (`Actor.K2_DestroyActor` _output))))

(fn `Get GM`
  (returns (GM :type "/Game/Blueprints/Managers/GM Object Reference"))
  (bind _outactors (`GameplayStatics.GetAllActorsOfClass` null "/Game/Blueprints/Managers/GM.GM_C"))
  (return (`|GetArrayItem` _outactors)))

(fn `Get Interactible Object that can be chosen by humans`
  (returns (`Interactible Objects Can Be Chosen By Humans` :type "Array of /Game/Blueprints/Entities/InteractibleObjects/InteractibleObject Object Reference"))
  (locals (`Interactible Objects Can Be Chosen By_Humans` :type "Array of /Game/Blueprints/Entities/InteractibleObjects/InteractibleObject Object Reference"))
  (bind _interactible_objects_can_be_chosen_by_humans (`local.Interactible Objects Can Be Chosen By_Humans`))
  (`KismetArrayLibrary.Array_Clear` (`local.Interactible Objects Can Be Chosen By_Humans`))
  (for _array_element (`self.Get InteractibleObjects` null)
    (if (`/Game/Blueprints/Entities/InteractibleObjects/InteractibleObject.Can Be Choose By Human` _array_element)
      (`KismetArrayLibrary.Array_Add` _interactible_objects_can_be_chosen_by_humans _array_element)))
  (return _interactible_objects_can_be_chosen_by_humans))

(fn `Get InteractibleObjects`
  (returns (`Interactible Objects` :type "Array of /Game/Blueprints/Entities/InteractibleObjects/InteractibleObject Object Reference"))
  (bind _outactors (`GameplayStatics.GetAllActorsOfClass` null "/Game/Blueprints/Entities/InteractibleObjects/InteractibleObject.InteractibleObject_C"))
  (return _outactors))

(fn `Get Player`
  (returns (Player :type "/Game/Blueprints/Entities/Player/Player Object Reference"))
  (bind _outactors (`GameplayStatics.GetAllActorsOfClass` null "/Game/Blueprints/Entities/Player/Player.Player_C"))
  (return (`|GetArrayItem` _outactors)))

(fn `Get Player Start`
  (returns (`Player start` :type "PlayerStart Object Reference"))
  (bind _outactors (`GameplayStatics.GetAllActorsOfClass` null "/Script/Engine.PlayerStart"))
  (return (`|GetArrayItem` _outactors)))

(fn `Get Random Spawn Point`
  (returns (`Random Spawn Point` :type "Actor Object Reference"))
  (bind _outactors (`GameplayStatics.GetAllActorsOfClass` null "/Game/Blueprints/Entities/IA/SpawnPointHumanNord.SpawnPointHumanNord_C"))
  (bind _outactors_2 (`GameplayStatics.GetAllActorsOfClass` null "/Game/Blueprints/Entities/IA/SpawnPointHumanSud.SpawnPointHumanSud_C"))
  (switch `int` (`KismetMathLibrary.RandomIntegerInRange` 0 1)
    (:`0`
      (return (`KismetArrayLibrary.Array_Random` _outactors)))
    (:`1`
      (return (`KismetArrayLibrary.Array_Random` _outactors_2)))))

(fn `Get Sound Manager`
  (returns (`Sound Manager` :type "/Game/Blueprints/Managers/SoundManager Object Reference"))
  (bind _outactors (`GameplayStatics.GetAllActorsOfClass` null "/Game/Blueprints/Managers/SoundManager.SoundManager_C"))
  (return (`|GetArrayItem` _outactors)))

(fn `Get State Processor`
  (returns (`State Processor` :type "/Game/Blueprints/Managers/StateProcessor Object Reference"))
  (bind _outactors (`GameplayStatics.GetAllActorsOfClass` null "/Game/Blueprints/Managers/StateProcessor.StateProcessor_C"))
  (return (`|GetArrayItem` _outactors)))

(fn `Get Waves Manager`
  (returns (`Waves Manager` :type "/Game/Blueprints/Managers/Waves/WavesManager Object Reference"))
  (bind _outactors (`GameplayStatics.GetAllActorsOfClass` null "/Game/Blueprints/Managers/Waves/WavesManager.WavesManager_C"))
  (return (`|GetArrayItem` _outactors)))

(fn `Is Human`
  (params (Human :type "Object Object Reference"))
  (returns (AsHuman :type "/Game/Blueprints/Entities/IA/Human Object Reference") (Success :type Boolean))
  (bind _ashuman (cast `/Game/Blueprints/Entities/IA/Human` Human)
    (:`then`
      (return _ashuman true))
    (:`CastFailed`
      (return _ashuman false))))

(fn `Is Interactible Object`
  (params (`Interactible Object` :type "Object Object Reference"))
  (returns (`As Interactible Object` :type "/Game/Blueprints/Entities/InteractibleObjects/InteractibleObject Object Reference") (Success :type Boolean))
  (bind _asinteractible_object (cast `/Game/Blueprints/Entities/InteractibleObjects/InteractibleObject` `Interactible Object`)
    (:`then`
      (return _asinteractible_object true))
    (:`CastFailed`
      (return _asinteractible_object false))))

(fn `Is Player`
  (params (Player :type "Object Object Reference"))
  (returns (`AsPlayer BP` :type "Object Object Reference") (Success :type Boolean))
  (bind _asplayer (cast `/Game/Blueprints/Entities/Player/Player` Player)
    (:`then`
      (return _asplayer true))
    (:`CastFailed`
      (return _asplayer false))))

(fn `Is Wall`
  (params (Wall :type "Object Object Reference"))
  (returns (Success :type Boolean) (`As Wall` :type "Object Object Reference"))
  (return false null))