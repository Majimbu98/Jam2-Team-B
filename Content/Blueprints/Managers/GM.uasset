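; GM is the game manager that runs a match where scaring people scores points and a person wanting to buy ends the game.
; On start it spawns and initializes the wave and state managers, adds the HUD and shows a paused tutorial once, tracked in the GameInstance.
; It also toggles the pause menu and, on loss, formats elapsed time, saves any new top score and shows the end screen.
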(event `Start New Game`
  (set `self.My Start Time` (`KismetMathLibrary.Now`))
  (`self.Spawn Other Managers`)
  (`/Game/Blueprints/Components/GodMode.Change God Mode` (`self.GodMode`))
  (`self.Set Starting Values`)
  (`/Game/Blueprints/Managers/StateProcessor.Set Interactible Object` (`/Game/Blueprints/Managers/Library.Get State Processor`))
  (`/Game/Blueprints/Managers/Waves/WavesManager.Activate` (`/Game/Blueprints/Managers/Library.Get Waves Manager`))
  (bind _asgame_instance (cast `/Game/Maps/GameInstance` (`GameplayStatics.GetGameInstance`)))
  (if (`/Game/Maps/GameInstance.Is Already opened Tutorial` _asgame_instance)
    (set `PlayerController.bShowMouseCursor` false (`GameplayStatics.GetPlayerController` 0))
    (else
      (bind _returnvalue (`|CreateWidget` "/Game/Widgets/Tutorial.Tutorial_C"))
      (`UserWidget.AddToViewport` _returnvalue 0)
      (set `/Game/Maps/GameInstance.Is Already opened Tutorial` true _asgame_instance)
      (`KismetSystemLibrary.Delay` 0.2)
      (`GameplayStatics.SetGamePaused` true)))
  (bind _returnvalue_2 (`|CreateWidget` "/Game/Widgets/UI.UI_C"))
  (set `self.My UI` _returnvalue_2)
  (`UserWidget.AddToViewport` _returnvalue_2 0))

(event `End Game`
  (`self.Lose Condition`))

(event `Person Want To Buy`
  (params (Human :type "/Game/Blueprints/Entities/IA/Human Object Reference"))
  (`self.End Game`))

(event `Person Scared!`
  (params (Human :type "/Game/Blueprints/Entities/IA/Human Object Reference"))
  (`/Engine/EditorBlueprintResources/StandardMacros.IncrementFloat` (`self.Current Score`)))

(event `Pause`
  (`self.Pause_Game`))

(fn `Calculate Time into Minutes and Second`
  (returns (`String Time` :type String))
  (bind _my_time (`self.My Time`))
  (set `self.My Time` (- (`KismetMathLibrary.Now`) (`self.My Start Time`)))
  (return (`KismetStringLibrary.Concat_StrStr` (`self.String Time`) (`KismetTextLibrary.Conv_TextToString` (`KismetTextLibrary.Conv_IntToText` (`KismetMathLibrary.GetMinutes` _my_time) false true 2)) ":" (`KismetTextLibrary.Conv_TextToString` (`KismetTextLibrary.Conv_IntToText` (`KismetMathLibrary.GetSeconds` _my_time) false true 2)))))

(fn `Lose Condition`
  (set `self.CountTime` false)
  (bind _string_time (`self.Calculate Time into Minutes and Second`))
  (set `self.String Time` _string_time)
  (set `self.EndGameScreen` true)
  (bind _output_get (set `self.New Top Score` (>= (`self.Current Score`) (`self.TopScore`))))
  (if _output_get
    (bind _output_get_2 (set `self.TopScore` (`self.Current Score`)))
    (set `/Game/Blueprints/Managers/MySaveGame.TopScore` _output_get_2 (`self.MySaveGameRef`))
    (`GameplayStatics.SaveGameToSlot` (`self.MySaveGameRef`) "MyGameSlot"))
  (bind _returnvalue (`|CreateWidget` "/Game/Widgets/EndGame.EndGame_C" (`GameplayStatics.GetPlayerController` 0)))
  (set `self.EndGame Ref` _returnvalue)
  (`UserWidget.AddToViewport` (`self.EndGame Ref`) 0)
  (set `PlayerController.bShowMouseCursor` true (`GameplayStatics.GetPlayerController` 0))
  (`WidgetBlueprintLibrary.SetInputMode_GameAndUIEx` (`GameplayStatics.GetPlayerController` 0) (`self.EndGame Ref`) "LockInFullscreen" false)
  (`GameplayStatics.SetGamePaused` true))

(fn `Pause_Game`
  (bind _returnvalue (`GameplayStatics.GetPlayerController` 0))
  (bind _returnvalue_2 (`GameplayStatics.GetCurrentLevelName` true))
  (if (and (`KismetStringLibrary.EqualEqual_StrStr` _returnvalue_2 "Game") (not (`self.EndGameScreen`)))
    (`/Engine/EditorBlueprintResources/StandardMacros.IsValid` (`self.Pause Ref`)
      (:`Is Valid`
        _)
      (:`Is Not Valid`
        (bind _returnvalue_3 (`|CreateWidget` "/Game/Widgets/Pause.Pause_C"))
        (set `self.Pause Ref` _returnvalue_3)))
    (if (`GameplayStatics.IsGamePaused`)
      (`Widget.RemoveFromParent` (`self.Pause Ref`))
      (`GameplayStatics.SetGamePaused` false)
      (`WidgetBlueprintLibrary.SetInputMode_GameOnly` _returnvalue)
      (set `PlayerController.bShowMouseCursor` false _returnvalue)
      (else
        (`UserWidget.AddToViewport` (`self.Pause Ref`) 0)
        (`GameplayStatics.SetGamePaused` true)
        (set `PlayerController.bShowMouseCursor` true (`GameplayStatics.GetPlayerController` 0))
        (`WidgetBlueprintLibrary.SetInputMode_GameAndUIEx` (`GameplayStatics.GetPlayerController` 0) (`self.Pause Ref`) "LockInFullscreen" false)))))

(fn `Set Starting Values`)

(fn `Spawn Other Managers`
  (locals (`Managers Number` :type Integer :default 2))
  (for _index (range (+ (`local.Managers Number`) 1))
    (`|SpawnActorFromClass` (select `int` _index :`0` null :`1` "/Game/Blueprints/Managers/Waves/WavesManager.WavesManager_C" :`2` "/Game/Blueprints/Managers/StateProcessor.StateProcessor_C" :!type "Actor Class Reference") (`SceneComponent.K2_GetComponentToWorld` (`self.DefaultSceneRoot`)) "Undefined" "OverrideRootScale" null null)))

(fn `UserConstructionScript`)